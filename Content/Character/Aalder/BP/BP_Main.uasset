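; BP_Main is the Aalder character Blueprint, handling the player's interact and pause inputs.
; Interact scans overlapping actors and sends InteractMessage to the first one that implements BI_InteractionInterface.
; Pause creates the WBP_UI_PauseMenu widget, adds it to the viewport, shows the cursor, switches to UI-only input and pauses the game.
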(event `self.ReceiveBeginPlay`)

(event `EnhancedInput|/Game/Input/Actions/IA_Interact`
  (params (ActionValue :type Boolean) (ElapsedSeconds :type "Float (double-precision)") (TriggeredSeconds :type "Float (double-precision)") (InputAction :type "InputAction Object Reference" :default "/Game/Input/Actions/IA_Interact.IA_Interact"))
  ;[1 1 1] Interact
  (:`Triggered`
    (for _array_element (`self.GetOverlappingActors` "/Script/Engine.Actor")
      (if (`KismetSystemLibrary.DoesImplementInterface` _array_element "/Game/Blueprints/Checkpoint/BI_InteractionInterface.BI_InteractionInterface_C")
        (message `/Game/Blueprints/Checkpoint/BI_InteractionInterface.Interact` _array_element)
        (break)))))

(event `EnhancedInput|/Game/Input/Actions/IA_Pause`
  (params (ActionValue :type Boolean) (ElapsedSeconds :type "Float (double-precision)") (TriggeredSeconds :type "Float (double-precision)") (InputAction :type "InputAction Object Reference" :default "/Game/Input/Actions/IA_Pause.IA_Pause"))
  (bind _returnvalue (`GameplayStatics.GetPlayerController` 0))
  (:`Started`
    (bind _returnvalue_2 (`|CreateWidget` "/Game/Blueprints/HUD/WBP_UI_PauseMenu.WBP_UI_PauseMenu_C"))
    (`UserWidget.AddToViewport` _returnvalue_2 0)
    (set `PlayerController.bShowMouseCursor` true _returnvalue)
    (`WidgetBlueprintLibrary.SetInputMode_UIOnlyEx` _returnvalue null)
    (`GameplayStatics.SetGamePaused` true)))

(fn `UserConstructionScript`)