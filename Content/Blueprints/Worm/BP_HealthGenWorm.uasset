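; BP_HealthGenWorm is a worm health pickup that heals an AalderPlayerCharacter through HealUpMaxHealth.
; A sphere overlap shows its widget to the player while IsActive is false, and hides it when active or when the player leaves.
; AddHealth heals the passed-in player, then destroys the worm after a brief delay.
; The worm mesh's custom depth rendering is switched off at BeginPlay.
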(event `self.ReceiveBeginPlay`
  (`PrimitiveComponent.SetRenderCustomDepth` (`self.SM_Worm`) false))

(event `self.SphereCollision.OnComponentBeginOverlap`
  (params (OverlappedComponent :type "PrimitiveComponent Object Reference") (OtherActor :type "Actor Object Reference") (OtherComp :type "PrimitiveComponent Object Reference") (OtherBodyIndex :type Integer) (bFromSweep :type Boolean) (SweepResult :type "HitResult Structure (by ref)"))
  (bind _widget (`self.Widget`))
  ;[1 1 1] Text Widget
  (cast `AalderPlayerCharacter` OtherActor)
  (if (`self.IsActive`)
    (`SceneComponent.SetVisibility` _widget false false :!label _label)
    (else
      (`SceneComponent.SetVisibility` _widget true false))))

(event `self.SphereCollision.OnComponentEndOverlap`
  (params (OverlappedComponent :type "PrimitiveComponent Object Reference") (OtherActor :type "Actor Object Reference") (OtherComp :type "PrimitiveComponent Object Reference") (OtherBodyIndex :type Integer))
  ;[1 1 1] Text Widget
  (cast `AalderPlayerCharacter` OtherActor)
  (goto _label))

(event `/Game/Blueprints/Checkpoint/BI_InteractionInterface.AddHealth`
  (params (Player :type "AalderPlayerCharacter Object Reference") (HUD :type "HUD Object Reference"))
  ;[1 1 1] Activate particles
  (`AalderPlayerCharacter.HealUpMaxHealth` Player)
  (`KismetSystemLibrary.Delay` 0.1)
  (`self.K2_DestroyActor`))

(fn `UserConstructionScript`)