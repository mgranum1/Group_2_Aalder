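; Interactable gate that shows a prompt widget to the player and slides down when used.
; Box overlaps with the player character show the widget on entry while the gate is unused, and hide it on exit.
; Interact plays a timeline from the start that lowers the gate mesh, setting IsActive and hiding the widget on each update.
; Interact does not check IsActive, so repeated calls replay the motion.
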(event `self.Box.OnComponentBeginOverlap`
  (params (OverlappedComponent :type "PrimitiveComponent Object Reference") (OtherActor :type "Actor Object Reference") (OtherComp :type "PrimitiveComponent Object Reference") (OtherBodyIndex :type Integer) (bFromSweep :type Boolean) (SweepResult :type "HitResult Structure (by ref)"))
  (bind _widget (`self.Widget`))
  ;[1 1 1] Text Widget
  (cast `AalderPlayerCharacter` OtherActor)
  (if (`self.IsActive`)
    (`SceneComponent.SetVisibility` _widget false false :!label _label)
    (else
      (`SceneComponent.SetVisibility` _widget true false))))

(event `self.Box.OnComponentEndOverlap`
  (params (OverlappedComponent :type "PrimitiveComponent Object Reference") (OtherActor :type "Actor Object Reference") (OtherComp :type "PrimitiveComponent Object Reference") (OtherBodyIndex :type Integer))
  ;[1 1 1] Text Widget
  (cast `AalderPlayerCharacter` OtherActor)
  (goto _label))

(event `/Game/Blueprints/Checkpoint/BI_InteractionInterface.Interact`
  (bind (_direction _doorfloat) (`Timeline|Timeline` :!via `PlayFromStart`)
    (:`Update`
      (`SceneComponent.K2_SetRelativeLocation` (`self.SM_Gate`) (`KismetMathLibrary.MakeVector` 0.0 0.0 (`KismetMathLibrary.Lerp` 0.0 -490.0 _doorfloat)) false false)
      (set `self.IsActive` true)
      (`SceneComponent.SetVisibility` (`self.Widget`) false false))))

(fn `UserConstructionScript`)