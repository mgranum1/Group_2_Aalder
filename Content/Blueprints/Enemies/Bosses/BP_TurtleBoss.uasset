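; BP_TurtleBoss is a boss enemy that stays hidden until activated and loads the win screen level when destroyed.
; It hides on BeginPlay, then Tick polls TurtleBossActive and, while true, unhides the boss and enables shooting every frame.
; ShootProjectile spawns a BP_ProjectileTurtle at the SpawnPoint's location and rotation if CanShoot is set; nothing in this Blueprint calls it.
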(event `self.ReceiveBeginPlay`
  (`self.SetActorHiddenInGame` true))

(event `self.ReceiveTick`
  (params (DeltaSeconds :type "Float (single-precision)"))
  (if (`self.TurtleBossActive`)
    (`self.SetActorHiddenInGame` false)
    (set `self.CanShoot` true)))

(event `self.ReceiveDestroyed`
  (`GameplayStatics.OpenLevel` "LVL_WinScreen"))

(fn `ShootProjectile`
  (locals (NewLocalVar :type "Float (single-precision)" :default -500.0))
  (if (`self.CanShoot`)
    (`|SpawnActorFromClass` "/Game/Blueprints/Weapons/BP_ProjectileTurtle.BP_ProjectileTurtle_C" (`KismetMathLibrary.MakeTransform` (.location (`SceneComponent.K2_GetComponentToWorld` (`self.SpawnPoint`))) (.rotation (`SceneComponent.K2_GetComponentToWorld` (`self.SpawnPoint`)))) "Undefined" "MultiplyWithRoot" null null)))

(fn `UserConstructionScript`)