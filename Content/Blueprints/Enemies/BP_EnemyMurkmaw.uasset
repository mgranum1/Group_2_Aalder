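; BP_EnemyMurkmaw is an enemy actor whose destruction opens the LVL_WinScreen level.
; On BeginPlay it stores the actor tagged "Player", keeping the last one found.
; ShootProjectile spawns a BP_Projectile at the enemy's transform, but nothing in this Blueprint calls it.
; Tick is empty, and a disconnected branch that would copy the player's rotation onto the enemy never runs.
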(event `self.ReceiveBeginPlay`
  (bind _outactors (`GameplayStatics.GetAllActorsWithTag` "Player"))
  (for _array_element _outactors
    (set `self.PlayerCharacter` _array_element)))

(event `self.ReceiveTick`
  (params (DeltaSeconds :type "Float (single-precision)")))

(event `self.ReceiveDestroyed`
  (`GameplayStatics.OpenLevel` "LVL_WinScreen"))

(fn `ShootProjectile`
  (`|SpawnActorFromClass` "/Game/Blueprints/Weapons/BP_Projectile.BP_Projectile_C" (`self.GetTransform`) "Undefined" "MultiplyWithRoot" null null))

(fn `UserConstructionScript`)