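; Water silhouette actor that travels along a spline path over a set duration.
; On BeginPlay it grabs the first BP_SplinePath actor in the level and starts a timeline, with play rate set to the inverse of TimeToCompleteSeconds.
; Each update maps the timeline track to distance along the spline and sets the actor transform, using world-space location but local-space rotation.
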(event `self.ReceiveBeginPlay`
  (bind _returnvalue (`GameplayStatics.GetActorOfClass` "/Game/Blueprints/WaterSilhouette/BP_SplinePath.BP_SplinePath_C"))
  (set `self.SplineRef` _returnvalue)
  (`self.MoveObject`))

(event `MoveObject`
  (bind _spline (`/Game/Blueprints/WaterSilhouette/BP_SplinePath.Spline` (`self.SplineRef`)))
  (`TimelineComponent.SetPlayRate` (`self.Move Object Timeline`) (/ 1.0 (`self.Time To Complete (Seconds)`)))
  (bind (_direction _movetrack) (`Timeline|Move Object Timeline`)
    (:`Update`
      (bind _returnvalue (`KismetMathLibrary.Lerp` 0.0 (`SplineComponent.GetSplineLength` (`/Game/Blueprints/WaterSilhouette/BP_SplinePath.Spline` (`self.SplineRef`))) _movetrack))
      (`self.K2_SetActorTransform` (`KismetMathLibrary.MakeTransform` (`SplineComponent.GetLocationAtDistanceAlongSpline` _spline _returnvalue "World") (`SplineComponent.GetRotationAtDistanceAlongSpline` _spline _returnvalue "Local"))))))

(fn `UserConstructionScript`)