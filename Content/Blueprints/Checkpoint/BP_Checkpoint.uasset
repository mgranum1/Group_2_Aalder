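; Interactable checkpoint stump that registers itself as the player's active checkpoint.
; Sphere overlap with the player character shows a prompt widget unless IsActive is set, and hides it on exit.
; Interact hides the widget, fires heart-leaf particles, swaps a stump material to a glowing one, and stores itself on BP_Main.
; Interact sets IsActive true but clears it again before registering, so the prompt can reappear.
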(event `self.SphereCollision.OnComponentBeginOverlap`
  (params (OverlappedComponent :type "PrimitiveComponent Object Reference") (OtherActor :type "Actor Object Reference") (OtherComp :type "PrimitiveComponent Object Reference") (OtherBodyIndex :type Integer) (bFromSweep :type Boolean) (SweepResult :type "HitResult Structure (by ref)"))
  (bind _widget (`self.Widget`))
  ;[1 1 1] Text Widget
  (cast `AalderPlayerCharacter` OtherActor)
  (if (`self.IsActive`)
    (`SceneComponent.SetVisibility` _widget false false :!label _label)
    (else
      (`SceneComponent.SetVisibility` _widget true false))))

(event `self.SphereCollision.OnComponentEndOverlap`
  (params (OverlappedComponent :type "PrimitiveComponent Object Reference") (OtherActor :type "Actor Object Reference") (OtherComp :type "PrimitiveComponent Object Reference") (OtherBodyIndex :type Integer))
  ;[1 1 1] Text Widget
  (cast `AalderPlayerCharacter` OtherActor)
  (goto _label))

(event `/Game/Blueprints/Checkpoint/BI_InteractionInterface.Interact`
  ;[1 1 1] Activate particles
  (set `self.IsActive` true)
  (`SceneComponent.SetVisibility` (`self.Widget`) false false)
  (`ActorComponent.Activate` (`self.HeartLeavesBurst`) false)
  (`PrimitiveComponent.SetMaterial` (`self.Stump`) 1 "/Game/Assets/CustomMade/Materials/M_Checkpoint_Wood_Glow_Inst.M_Checkpoint_Wood_Glow_Inst")
  (`ActorComponent.Activate` (`self.HeartLeaves`) false)
  (set `self.IsActive` false)
  (bind _asbp_main (cast `/Game/Character/Aalder/BP/BP_Main` (`GameplayStatics.GetPlayerPawn` 0)))
  (set `/Game/Character/Aalder/BP/BP_Main.ActiveCheckpoint` self _asbp_main))

(fn `UserConstructionScript`)